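; Zombie factory actor that spawns a BP_Zombie whenever the first-person character's Recargar (reload) event fires.
; On BeginPlay it binds SpawnZombie to that event on the player character.
; Each zombie spawns at a hard-coded location and is assigned the DA_ZombieLent data asset after spawning.
; UpdateZombie then gives its cylinder mesh a dynamic MI_Zombie material tinted with the data asset's color.
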(event `self.ReceiveBeginPlay`
  (bind _asbp_first_person_character (cast `/Game/FirstPerson/Blueprints/BP_FirstPersonCharacter` (`GameplayStatics.GetPlayerCharacter` 0)))
  (add `/Game/FirstPerson/Blueprints/BP_FirstPersonCharacter.Recargar` _asbp_first_person_character (delegate `SpawnZombie`)))

(event `SpawnZombie`
  (bind _returnvalue (`|SpawnActorFromClass` "/Game/MyFolder/Zombie/BP_Zombie.BP_Zombie_C" (`KismetMathLibrary.MakeTransform` (1500.0 50.0 150.0)) "AdjustIfPossibleButAlwaysSpawn" "MultiplyWithRoot" null null))
  (set `/Game/MyFolder/Zombie/BP_Zombie.ZombieData` "/Game/MyFolder/Zombie/DA_ZombieLent.DA_ZombieLent" _returnvalue)
  (`self.UpdateZombie` _returnvalue))

(fn `UpdateZombie`
  (params (Zombie :type "/Game/MyFolder/Zombie/BP_Zombie Object Reference"))
  (bind _returnvalue (`PrimitiveComponent.CreateDynamicMaterialInstance` (`/Game/MyFolder/Zombie/BP_Zombie.Cylinder` Zombie) 0 "/Game/MyFolder/Zombie/MI_Zombie.MI_Zombie" "None"))
  (`MaterialInstanceDynamic.SetVectorParameterValue` _returnvalue "Color" (`KismetMathLibrary.Conv_ColorToLinearColor` (`/Game/MyFolder/Zombie/UData_Zombie.Color` (`/Game/MyFolder/Zombie/BP_Zombie.ZombieData` Zombie)))))

(fn `UserConstructionScript`)